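; Game mode for the ragdoll game that sets up the match, detects victory and handles game over.
; On BeginPlay it loads or creates the difficulty save object, sets game-only input and adds the player HUD.
; Tick polls for remaining gummy and bear gummy enemies, showing the win screen once when none are left.
; ShowEndScreen flags game over, displays the win/loss widget, switches to UI-only input and ignores movement.
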(event Custom|ShowEndScreen
  (params (WonGame :type Boolean))
  (bind _returnvalue (Game|GetPlayerController 0))
  ;[0.06301 0.06301 0.06301] Display the end screen and allow the player to click things on the end screen.
  (Variables|Default|SetIsGameOver true)
  (bind _returnvalue_2 (UserInterface|CreateWidget "/Game/Blueprints/UI/WBP_EndScreen.WBP_EndScreen_C" 0 WonGame))
  (bind _output_get (Variables|Default|SetEndScreenRef _returnvalue_2))
  (UserInterface|Viewport|AddtoViewport _output_get 0)
  (Input|SetInputModeUIOnly _returnvalue _output_get "DoNotLock" false)
  (Variables|/Script/Engine.PlayerController|SetbShowMouseCursor _returnvalue true)
  (Input|SetIgnoreMoveInput _returnvalue true))

(event EventBeginPlay
  ;[0.06301 0.06301 0.06301] Get a reference to the difficulty settings save data, ensure the input mode is game only, and add the player HUD widget to the viewport.
  (CallFunction|LoadDifficultySettings)
  (Input|SetInputModeGameOnly (Game|GetPlayerController 0) false)
  (bind _returnvalue (UserInterface|CreateWidget "/Game/Blueprints/UI/WBP_PlayerHUD.WBP_PlayerHUD_C"))
  (bind _output_get (Variables|Default|SetPlayerHUD _returnvalue))
  (UserInterface|Viewport|AddtoViewport _output_get 0))

(event EventTick
  (params (DeltaSeconds :type Float%20%28single-precision%29))
  ;[0.06301 0.06301 0.06301] If there are no enemies, display the win screen.
  (bind _outactors (Actor|GetAllActorsOfClass "/Game/Blueprints/AI/BP_EnemyGummy_Child.BP_EnemyGummy_Child_C"))
  (if (not (>= (Utilities|Array|Length _outactors) 1))
    (bind _outactors_2 (Actor|GetAllActorsOfClass "/Game/Blueprints/BP_BearEnemyGummy.BP_BearEnemyGummy_C"))
    (if (not (>= (Utilities|Array|Length _outactors_2) 1))
      (Utilities|FlowControl|DoOnce false
        (:Completed
          (CallFunction|ShowEndScreen true))))))

(fn ConstructionScript)

(fn LoadDifficultySettings
  (bind _returnvalue (SaveGame|DoesSaveGameExist (Variables|SaveData|Difficulty|GetDifficultySaveFileName)))
  (if _returnvalue
    (bind _returnvalue_2 (SaveGame|LoadGamefromSlot (Variables|SaveData|Difficulty|GetDifficultySaveFileName)))
    (bind _asbp_difficulty_settings (Utilities|Casting|CastToBP_DifficultySettings _returnvalue_2))
    (Variables|SaveData|Difficulty|SetDifficultySaveData _asbp_difficulty_settings)
    (else
      (bind _returnvalue_3 (SaveGame|CreateSaveGameObject "/Game/Blueprints/Saving/BP_DifficultySettings.BP_DifficultySettings_C"))
      (Variables|SaveData|Difficulty|SetDifficultySaveData _returnvalue_3))))