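; Gummy bear enemy that roams randomly as an active ragdoll (physical animation) and damages BP_GummyBear through a per-tick club sphere trace.
; EnemyLoseHealth removes one health per accepted hit, updates the camera-facing health bar, then fully ragdolls and destroys the bear at zero.
; The damage cooldown starts only when a blocked hit arrives.
; Per-bone dismemberment functions are not called here, and the zombie crawl logic is disconnected.
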(event Custom|RandomRoam
  ;[0.06301 0.06301 0.06301] Random roam
  (AI|AIMoveTo self (.RandomLocation (AI|Navigation|GetRandomReachablePointinRadius (Transformation|GetActorLocation) 5e+03 0 0)) 0 5.0 false
    (:OnSuccess
      _)
    (:OnFail
      _))
  (CallFunction|RandomRoam))

(event Custom|EnemyLoseHealth
  (params (Damage :type Integer) (HitBoneName :type Name) (DamageCauser :type Actor%20Object%20Reference))
  (bind _mesh (Variables|Character|GetMesh))
  ;[0.06301 0.06301 0.06301] Enemy takes damage when hit and cooldown is at 0. If the enemy health hits 0, the enemy will ragdoll and the end screen will show up with a victory message.
  (if (Variables|Default|GetCanTakeDamage)
    (Variables|Default|SetCanTakeDamage false)
    (Private|PlayTakeDamageSound)
    (bind _result (Math|Integer|DecrementInt (Variables|Default|GetEnemyHealth))
      (:%20%20
        (Variables|Default|SetEnemyHealth _result)
        (Private|UpdateHealthBar)
        (if (<= (Variables|Default|GetEnemyHealth) 0)
          (Collision|SetCollisionEnabled _mesh "QueryAndPhysics")
          (Physics|SetSimulatePhysics _mesh true)
          (Class|SkeletalMeshComponent|SetPhysicsBlendWeight _mesh 1.0)
          (bind _healthbarwidget (Variables|Default|GetHealthBarWidget)
            (:then
              (Components|DestroyComponent _healthbarwidget))
            (:else
              _))
          (Utilities|FlowControl|Delay 3.0)
          (Actor|DestroyActor))))
    (else
      (Utilities|FlowControl|Delay (Variables|Default|GetPlayerCooldown))
      (Variables|Default|SetCanTakeDamage true))))

(event EventTick
  (params (DeltaSeconds :type Float%20%28single-precision%29))
  (CallFunction|EnemyHitDetect)
  (Private|HealthBarFacePlayer))

(event EventBeginPlay
  ;[0.05286 0.05286 0.05286] Set reference to the gamemode.
  (bind _asgm_ragdoll_game (Utilities|Casting|CastToGM_RagdollGame (Game|GetGameMode)))
  (Variables|Default|SetGMRef _asgm_ragdoll_game)
  (CallFunction|RandomRoam)
  (Private|BeginPlay|ActiveRagdoll)
  (bind _aswbp_health_bar (Utilities|Casting|CastToWBP_HealthBar (UserInterface|GetWidget (Variables|Default|GetHealthBarWidget))))
  (Variables|Private|UI|SetWBP_HealthBar _aswbp_health_bar))

(fn ConstructionScript)

(fn EnemyHitDetect
  (bind _club (Variables|Default|GetClub))
  (bind _outhit (Collision|SphereTraceForObjects (Transformation|GetSocketLocation _club "Start") (Transformation|GetSocketLocation _club "End") 15.0 (Utilities|Array|MakeArray "ObjectTypeQuery3") false 0 "None"))
  (bind _asbp_gummy_bear (Utilities|Casting|CastToBP_GummyBear (.HitActor (Collision|BreakHitResult _outhit))))
  (Default|LoseHealth _asbp_gummy_bear))

(fn AnyDamage
  (params (Damage :type Integer) (HitBoneName :type Name) (DamageCauser :type Actor%20Object%20Reference))
  (Variables|Default|SetAppliedDamage Damage)
  (Variables|Default|SetHit%20Bone%20Name HitBoneName)
  (Variables|Default|SetDamage%20Causer DamageCauser)
  (CallFunction|RenameBoneName)
  (bind _reacheddurabilitylimit (CallFunction|ApplyDamagetoBone))
  (if _reacheddurabilitylimit
    (CallFunction|Dismemberment)
    (CallFunction|ChangeMovementType)
    (CallFunction|ApplyPhysics)))

(fn RenameBoneName
  (switch name (Variables|Default|GetHit%20Bone%20Name)
    (:Pelvis
      _)
    (:Spine_02
      _)
    (:Spine_03
      _)
    (:Neck_01
      _)
    (:Head
      _))
  (Variables|Default|SetHit%20Bone%20Name "spine_01"))

(fn ApplyDamagetoBone
  (bind _breakablebones_durability (Variables|Default|GetBreakableBones/Durability))
  (bind _hit_bone_name (Variables|Default|GetHit%20Bone%20Name))
  (bind (_value _returnvalue) (Utilities|Map|Find _breakablebones_durability _hit_bone_name))
  (if _returnvalue
    (Utilities|Map|Add (Variables|Default|GetBreakableBones/Durability) (Variables|Default|GetHit%20Bone%20Name) (- _value (Variables|Default|GetAppliedDamage)))
    (return (<= (.Value (Utilities|Map|Find (Variables|Default|GetBreakableBones/Durability) (Variables|Default|GetHit%20Bone%20Name))) 0))))

(fn Dismemberment
  (bind _hit_bone_name (Variables|Default|GetHit%20Bone%20Name))
  (bind _mesh (Variables|Character|GetMesh))
  (bind _mesh_2 (Variables|Character|GetMesh))
  (bind _hit_bone_name_2 (Variables|Default|GetHit%20Bone%20Name))
  (bind _hit_bone_name_3 (Variables|Default|GetHit%20Bone%20Name))
  (bind _returnvalue (Transformation|GetSocketTransform _mesh_2 _hit_bone_name "RTS_World"))
  (bind _returnvalue_2 (Transformation|GetWorldLocation _mesh))
  (Class|SkeletalMeshComponent|BreakConstraint (Variables|Character|GetMesh) (Utilities|CalculateImpulse) (Utilities|GetSocketLocation) _hit_bone_name)
  (Components|SkinnedMesh|HideBonebyName (Variables|Character|GetMesh) _hit_bone_name_2 "PBO_None")
  (Effects|SpawnEmitterAttached "/Engine/Tutorial/SubEditors/TutorialAssets/TutorialParticleSystem.TutorialParticleSystem" _mesh_2 _hit_bone_name_2 (.location _returnvalue) (.rotation _returnvalue) "0.100000,0.100000,0.100000" "KeepWorldPosition")
  (Effects|SpawnEmitterAttached "/Engine/Tutorial/SubEditors/TutorialAssets/TutorialParticleSystem.TutorialParticleSystem" (Variables|Character|GetMesh) (Variables|Default|GetHit%20Bone%20Name) (.location _returnvalue) (.rotation _returnvalue) "0.100000,0.100000,0.100000" "KeepWorldPosition")
  (Effects|SpawnEmitterAttached "/Engine/Tutorial/SubEditors/TutorialAssets/TutorialParticleSystem.TutorialParticleSystem" (Variables|Character|GetMesh) (Variables|Default|GetHit%20Bone%20Name) (.location _returnvalue) (.rotation _returnvalue) "0.100000,0.100000,0.100000" "KeepWorldPosition")
  (Variables|Default|SetHasSpineBroken (== _hit_bone_name_3 "spine_01"))
  (Utilities|Array|Add (Variables|Default|GetBrokenBones) _hit_bone_name_3)
  (bind _outhit (Collision|LineTraceByChannel _returnvalue_2 (+ _returnvalue_2 (* "0.000000,0.000000,-1.000000" 1e+03)) "TraceTypeQuery1" false 0 "None"))
  (Rendering|Decal|SpawnDecalatLocation 0 "-63.000000,-128.000000,-128.000000" (.Location (Collision|BreakHitResult _outhit)) (Math|Conversions|RotationFromXVector (.Normal (Collision|BreakHitResult _outhit))) 6e+01))

(fn ChangeMovementType
  (if (Utilities|Enum|Equal(Enum) (Variables|Default|GetMovementZombie) "NewEnumerator0")
    (Variables|Default|SetMovementZombie "NewEnumerator1")))

(fn ApplyPhysics
  (bind _mesh (Variables|Character|GetMesh))
  (switch name (Variables|Default|GetHit%20Bone%20Name)
    (:spine_01
      _)
    (:thigh_r
      _)
    (:thigh_l
      _)
    (:calf_r
      _)
    (:calf_l
      _)
    (:foot_r
      _)
    (:foot_l
      _)
    (:head
      _))
  (Physics|SetSimulatePhysics _mesh true)
  (Physics|AddImpulseatLocation _mesh (Utilities|CalculateImpulse) (Utilities|GetSocketLocation) (Variables|Default|GetHit%20Bone%20Name))
  (Collision|SetCollisionEnabled (Variables|Collision|GetCapsuleComponent) "NoCollision"))

(fn SetCapsuleLocation
  (Transformation|SetWorldLocation (Variables|Collision|GetCapsuleComponent) (Transformation|GetSocketLocation (Variables|Character|GetMesh) "head") false false))

(fn AddForcetoBones
  (Physics|AddForce (Variables|Character|GetMesh) (Utilities|CalculateCrawlForce 5e+02 3e+03) "head" true)
  (Utilities|FindBrokenBones (Utilities|Array|MakeArray "upperarm_r" "lowerarm_r" "hand_r")
    (:true
      _)
    (:false
      (Physics|AddForce (Variables|Character|GetMesh) (Utilities|CalculateCrawlForce 1e+03 1e+03) "hand_r" true)))
  (Utilities|FindBrokenBones (Utilities|Array|MakeArray "upperarm_l" "lowerarm_l" "hand_l")
    (:false
      (Physics|AddForce (Variables|Character|GetMesh) (Utilities|CalculateCrawlForce 1e+03 1e+03) "hand_l" true))))

(fn ActiveRagdoll
  (bind _boneclosesttoroot (Variables|Default|GetBoneClosestToRoot))
  (bind _physicalanimation (Variables|Default|GetPhysicalAnimation))
  ;[1 0.9615 0.7332] Active Ragdoll
  (Class|PhysicalAnimationComponent|SetSkeletalMeshComponent _physicalanimation (Variables|Character|GetMesh))
  (Class|PhysicalAnimationComponent|ApplyPhysicalAnimationSettingsBelow _physicalanimation _boneclosesttoroot (Utilities|Struct|MakePhysicalAnimationData true 1e+03 5e+02 1e+03 5e+02 5e+01 5e+01) true)
  (Class|SkeletalMeshComponent|SetAllBodiesBelowSimulatePhysics (Variables|Character|GetMesh) _boneclosesttoroot true false))

(fn UpdateHealthBar
  (Progress|SetPercent (Variables|/Game/Blueprints/HealthBars/WBP_HealthBar.WBP_HealthBar_C|GetHealthBar (Variables|Private|UI|GetWBP_HealthBar)) (/ (Variables|Default|GetEnemyHealth) (Variables|Private|Constant|GetEnemyMaxHealth))))

(fn HealthBarFacePlayer
  (bind _healthbarwidget (Variables|Default|GetHealthBarWidget)
    (:then
      (Transformation|SetWorldRotation _healthbarwidget (Math|Rotator|FindLookatRotation (Transformation|GetWorldLocation _healthbarwidget) (Transformation|GetWorldLocation (Variables|/Script/Engine.PlayerCameraManager|GetTransformComponent (Game|GetPlayerCameraManager 0)))) false false))
    (:else)))

(fn PlayTakeDamageSound
  (bind _damaged (Variables|Default|GetDamaged))
  (if (Utilities|IsAudioNotPlaying _damaged)
    (Audio|Components|Audio|Play _damaged 0.0))
  (return))