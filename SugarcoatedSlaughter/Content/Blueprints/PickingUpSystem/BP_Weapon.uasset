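; BP_Weapon is a placeable weapon pickup that shrinks away and removes itself when picked up.
; Its construction script applies the configurable WeaponModelToPlace mesh to the WeaponModel component.
; The PickUp event runs a timeline that scales the root component from full size down to zero.
; A DoOnce on the timeline's update plays the pickup sound once at the actor, then destroys it after a short delay.
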(event EventPickUp
  (bind _shrinktimeline (Timeline|ShrinkAnim Play)
    (:Update
      (Transformation|SetWorldScale3D (Variables|Default|GetDefaultSceneRoot) (Math|Conversions|ToVector(Float) (Math|Float|Lerp 1.0 0.0 _shrinktimeline)))
      (Utilities|FlowControl|DoOnce false
        (:Completed
          (Audio|PlaySoundatLocation "/Engine/VREditor/Sounds/UI/Object_PickUp.Object_PickUp" (Transformation|GetActorLocation) "0, 0, 0" 2.0 1.0 0.0 0 0 0 0)
          (Utilities|FlowControl|Delay 0.6)
          (Actor|DestroyActor))))))

(fn ConstructionScript
  (Components|StaticMesh|SetStaticMesh (Variables|Default|GetWeaponModel) (Variables|Default|GetWeaponModelToPlace)))