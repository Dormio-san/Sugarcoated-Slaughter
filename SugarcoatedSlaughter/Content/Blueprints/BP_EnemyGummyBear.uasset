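; Enemy gummy bear for the ragdoll game that roams randomly and hurts the player with its sword.
; It chains AI moves to random reachable points and sphere-traces along the sword sockets every tick, calling LoseHealth on any BP_GummyBear hit.
; Incoming hits remove health behind a cooldown flag, re-armed after a delay only when a blocked hit arrives.
; At zero health it ragdolls, is destroyed, and triggers the GameMode's victory screen.
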(event Custom|RandomRoam
  (AI|AIMoveTo self (.RandomLocation (AI|Navigation|GetRandomReachablePointinRadius (Transformation|GetActorLocation) 5e+03 0 0)) 0 5.0 false
    (:OnSuccess
      _)
    (:OnFail
      _))
  (CallFunction|RandomRoam))

(event Custom|EnemyLoseHealth
  (bind _skeletalmesh (Variables|Default|GetSkeletalMesh))
  ;[0.06301 0.06301 0.06301] Enemy takes damage when hit and cooldown is at 0. If the enemy health hits 0, the enemy will ragdoll and the end screen will show up with a victory message.
  (if (Variables|Default|GetCanTakeDamage)
    (Variables|Default|SetCanTakeDamage false)
    (bind _result (Math|Integer|DecrementInt (Variables|Default|GetEnemyHealth))
      (:%20%20
        (bind _output_get (Variables|Default|SetEnemyHealth _result))
        (Development|PrintString (Utilities|String|Append "Enemy Health: " (Utilities|String|ToString(Integer) _output_get)) true true "(R=0.249146,G=1.000000,B=0.000000,A=1.000000)" 3.0)
        (if (<= (Variables|Default|GetEnemyHealth) 0)
          (Collision|SetCollisionEnabled _skeletalmesh "QueryAndPhysics")
          (Physics|SetSimulatePhysics _skeletalmesh true)
          (Class|SkeletalMeshComponent|SetPhysicsBlendWeight _skeletalmesh 1.0)
          (Utilities|FlowControl|Delay 3.0)
          (Actor|DestroyActor)
          (Default|ShowEndScreen (Variables|Default|GetGMRef) true))))
    (else
      (Utilities|FlowControl|Delay (Variables|Default|GetPlayerCooldown))
      (Variables|Default|SetCanTakeDamage true))))

(event EventBeginPlay
  ;[0.06301 0.06301 0.06301] When the game begins, get a reference to the gamemode.
  (bind _asgm_ragdoll_game (Utilities|Casting|CastToGM_RagdollGame (Game|GetGameMode)))
  (Variables|Default|SetGMRef _asgm_ragdoll_game)
  (CallFunction|RandomRoam))

(event EventTick
  (params (DeltaSeconds :type Float%20%28single-precision%29))
  (CallFunction|EnemyHitDetect))

(fn ConstructionScript)

(fn EnemyHitDetect
  (bind _sword (Variables|Default|GetSword))
  (bind _outhit (Collision|SphereTraceForObjects (Transformation|GetSocketLocation _sword "Start") (Transformation|GetSocketLocation _sword "End") 1e+01 (Utilities|Array|MakeArray "ObjectTypeQuery3") false 0 "ForDuration"))
  (bind _asbp_gummy_bear (Utilities|Casting|CastToBP_GummyBear (.HitActor (Collision|BreakHitResult _outhit))))
  (Default|LoseHealth _asbp_gummy_bear))