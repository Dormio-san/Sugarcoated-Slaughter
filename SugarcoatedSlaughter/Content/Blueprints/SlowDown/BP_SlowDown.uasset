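; BP_SlowDown is a zone actor that scales the walk speed of any Character inside its BoxCollider.
; On begin overlap it saves the character's MaxWalkSpeed and multiplies it by WalkSpeedChangeAmount, so the multiplier decides whether it slows or speeds up.
; On end overlap it restores the saved speed, which lives in a single NormalWalkSpeed variable shared by all overlapping characters.
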(event OnComponentBeginOverlap(BoxCollider)
  (params (OverlappedComponent :type Primitive%20Component%20Object%20Reference) (OtherActor :type Actor%20Object%20Reference) (OtherComp :type Primitive%20Component%20Object%20Reference) (OtherBodyIndex :type Integer) (bFromSweep :type Boolean) (SweepResult :type Hit%20Result%20Structure%20%28by%20ref%29))
  ;[1 0.4564 0.0999] Speed up when in zone
  (bind _ascharacter (Utilities|Casting|CastToCharacter OtherActor))
  (Variables|Private|SetNormalWalkSpeed (Variables|/Script/Engine.CharacterMovementComponent|GetMaxWalkSpeed (Variables|/Script/Engine.Character|GetCharacterMovement _ascharacter)))
  (Variables|/Script/Engine.CharacterMovementComponent|SetMaxWalkSpeed (Variables|/Script/Engine.Character|GetCharacterMovement _ascharacter) (* (Variables|/Script/Engine.CharacterMovementComponent|GetMaxWalkSpeed (Variables|/Script/Engine.Character|GetCharacterMovement _ascharacter)) (Variables|Default|GetWalkSpeedChangeAmount))))

(event OnComponentEndOverlap(BoxCollider)
  (params (OverlappedComponent :type Primitive%20Component%20Object%20Reference) (OtherActor :type Actor%20Object%20Reference) (OtherComp :type Primitive%20Component%20Object%20Reference) (OtherBodyIndex :type Integer))
  ;[1 0.4564 0.0999] Set speed back to normal when exiting zone.
  (bind _ascharacter (Utilities|Casting|CastToCharacter OtherActor))
  (Variables|/Script/Engine.CharacterMovementComponent|SetMaxWalkSpeed (Variables|/Script/Engine.Character|GetCharacterMovement _ascharacter) (Variables|Private|GetNormalWalkSpeed)))

(fn ConstructionScript)