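; BP_EnemyGummy_Child is a child Blueprint of an enemy, apparently a gummy variant, that removes itself once its health is depleted.
; It runs the parent's logic, then sets PlayerHealth at BeginPlay.
; Tick polls that value and, at zero or below, destroys the actor after a short delay.
; Nothing in this graph reduces the health.
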(event EventBeginPlay
  (|CallParentFunction)
  (Variables|Default|SetPlayerHealth 3))

(event EventTick
  (params (DeltaSeconds :type Float%20%28single-precision%29))
  (|CallParentFunction DeltaSeconds)
  (if (<= (Variables|Default|GetPlayerHealth) 0)
    (Utilities|FlowControl|Delay 3.0)
    (Actor|DestroyActor)))

(fn ConstructionScript
  (|CallParentFunction))