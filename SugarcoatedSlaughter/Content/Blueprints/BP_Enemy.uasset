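; BP_Enemy is an enemy that loses health when hit and ragdolls on defeat in a ragdoll game.
; EnemyLoseHealth decrements health and prints it, gated by a CanTakeDamage flag that re-arms after a Cooldown delay started only by a blocked hit.
; At zero health, the skeletal mesh switches to physics simulation, the cached GM_RagdollGame shows the victory end screen, and the actor is destroyed shortly after.
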(event Custom|EnemyLoseHealth
  (bind _skm_quinn_simple (Variables|Default|GetSKM_Quinn_Simple))
  ;[0.06301 0.06301 0.06301] Enemy takes damage when hit and cooldown is at 0. If the enemy health hits 0, the enemy will ragdoll and the end screen will show up with a victory message.
  (if (Variables|Default|GetCanTakeDamage)
    (Variables|Default|SetCanTakeDamage false)
    (bind _result (Math|Integer|DecrementInt (Variables|Default|GetEnemyHealth))
      (:%20%20
        (bind _output_get (Variables|Default|SetEnemyHealth _result))
        (Development|PrintString (Utilities|String|Append "Enemy Health: " (Utilities|String|ToString(Integer) _output_get)) true true "(R=0.249146,G=1.000000,B=0.000000,A=1.000000)" 3.0)
        (if (<= (Variables|Default|GetEnemyHealth) 0)
          (Collision|SetCollisionEnabled _skm_quinn_simple "QueryAndPhysics")
          (Physics|SetSimulatePhysics _skm_quinn_simple true)
          (Class|SkeletalMeshComponent|SetPhysicsBlendWeight _skm_quinn_simple 1.0)
          (Default|ShowEndScreen (Variables|Default|GetGMRef) true)
          (Utilities|FlowControl|Delay 1.8)
          (Actor|DestroyActor))))
    (else
      (Utilities|FlowControl|Delay (Variables|Default|GetCooldown))
      (Variables|Default|SetCanTakeDamage true))))

(event EventBeginPlay
  ;[0.06301 0.06301 0.06301] When the game begins, get a reference to the gamemode.
  (bind _asgm_ragdoll_game (Utilities|Casting|CastToGM_RagdollGame (Game|GetGameMode)))
  (Variables|Default|SetGMRef _asgm_ragdoll_game))

(fn ConstructionScript)