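; Main-menu customization stage that spawns a BP_PlayerCapture preview character and edits its look.
; On BeginPlay it loads or creates the BP_SavedCustomizationData save object, without applying saved values to the preview.
; Click-and-drag yaws the preview, while functions swap weapon meshes, toggle hat visibility and randomize colors through dynamic material instances.
; Each change is written into the save object, and SaveGame commits it to the slot.
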(event Custom|MouseMove
  (params (Delta :type Vector%202D%20Structure))
  (if (Variables|Default|GetCanRotate)
    (Transformation|AddActorLocalRotation (Variables|Default|GetPlayerCaptureRef) (Math|Rotator|MakeRotator 0.0 0.0 (.X (Math|Vector2D|BreakVector2D (/ Delta (Variables|Default|GetRotateSpeed))))) false false)))

(event Custom|ClickedStart
  (Variables|Default|SetCanRotate true))

(event Custom|ClickedEnd
  (Variables|Default|SetCanRotate false))

(event EventBeginPlay
  (bind _returnvalue (Game|SpawnActorfromClass "/Game/MainMenu/CustomizationMenu/BP_PlayerCapture.BP_PlayerCapture_C" (Math|Transform|MakeTransform (Transformation|GetWorldLocation (Variables|Default|GetScene))) "AlwaysSpawn" "MultiplyWithRoot" 0 0))
  (Variables|Default|SetPlayerCaptureRef _returnvalue)
  (Variables|Default|SetPlayerHats (Utilities|Array|MakeArray (Variables|/Game/Blueprints/BP_GummyBear.BP_GummyBear_C|GetSkullHat_Low (Variables|Default|GetPlayerCaptureRef)) (Variables|/Game/Blueprints/BP_GummyBear.BP_GummyBear_C|GetHelmet (Variables|Default|GetPlayerCaptureRef)) (Variables|/Game/Blueprints/BP_GummyBear.BP_GummyBear_C|GetVikingHelmet (Variables|Default|GetPlayerCaptureRef))))
  (bind _returnvalue_2 (SaveGame|DoesSaveGameExist (Variables|Default|GetSaveFileName)))
  (if _returnvalue_2
    (bind _returnvalue_3 (SaveGame|LoadGamefromSlot (Variables|Default|GetSaveFileName)))
    (bind _asbp_saved_customization_data (Utilities|Casting|CastToBP_SavedCustomizationData _returnvalue_3))
    (Variables|Default|SetCustomizationSaveData _asbp_saved_customization_data)
    (else
      (bind _returnvalue_4 (SaveGame|CreateSaveGameObject "/Game/Blueprints/Saving/BP_SavedCustomizationData.BP_SavedCustomizationData_C"))
      (Variables|Default|SetCustomizationSaveData _returnvalue_4))))

(fn ConstructionScript)

(fn ChangeWeapon
  (params (WeaponName :type String))
  (bind _playercaptureref (Variables|Default|GetPlayerCaptureRef))
  (bind _playercaptureref_2 (Variables|Default|GetPlayerCaptureRef))
  (bind _playercaptureref_3 (Variables|Default|GetPlayerCaptureRef))
  (bind _playercaptureref_4 (Variables|Default|GetPlayerCaptureRef))
  (bind _output_get (Variables|/Game/Blueprints/Saving/BP_SavedCustomizationData.BP_SavedCustomizationData_C|SetSavedWeaponName (Variables|Default|GetCustomizationSaveData) WeaponName))
  (switch string _output_get
    (:Default
      (Components|StaticMesh|SetStaticMesh (Variables|/Game/Blueprints/BP_GummyBear.BP_GummyBear_C|GetEquippedWeapon _playercaptureref_2) 0)
      (Components|StaticMesh|SetStaticMesh (Variables|/Game/Blueprints/BP_GummyBear.BP_GummyBear_C|GetSwordWeapon _playercaptureref_2) 0))
    (:Sword
      (Components|StaticMesh|SetStaticMesh (Variables|/Game/Blueprints/BP_GummyBear.BP_GummyBear_C|GetSwordWeapon _playercaptureref) "/Game/Art/Sword/sword_low.sword_low")
      (Components|StaticMesh|SetStaticMesh (Variables|/Game/Blueprints/BP_GummyBear.BP_GummyBear_C|GetEquippedWeapon _playercaptureref) 0))
    (:Club
      (Components|StaticMesh|SetStaticMesh (Variables|/Game/Blueprints/BP_GummyBear.BP_GummyBear_C|GetEquippedWeapon _playercaptureref_4) "/Game/Art/Props/Club.Club")
      (Components|StaticMesh|SetStaticMesh (Variables|/Game/Blueprints/BP_GummyBear.BP_GummyBear_C|GetSwordWeapon _playercaptureref_4) 0))
    (:Spear
      (Components|StaticMesh|SetStaticMesh (Variables|/Game/Blueprints/BP_GummyBear.BP_GummyBear_C|GetEquippedWeapon _playercaptureref_3) 0)
      (Components|StaticMesh|SetStaticMesh (Variables|/Game/Blueprints/BP_GummyBear.BP_GummyBear_C|GetSwordWeapon _playercaptureref_3) "/Game/Art/Props/spear_low.spear_low"))))

(fn RandomColor
  (bind _customizationsavedata (Variables|Default|GetCustomizationSaveData))
  (bind _returnvalue (Rendering|Material|CreateDynamicMaterialInstance (Variables|/Script/Engine.Character|GetMesh (Variables|Default|GetPlayerCaptureRef)) 0 0 "None" :!class /Script/Engine.PrimitiveComponent))
  (bind _output_get (LocalVariables|SetColor1 (Utilities|Struct|MakeLinearColor (Math|Random|RandomFloat) (Math|Random|RandomFloat) (Math|Random|RandomFloat) 1.0)))
  (Rendering|Material|SetVectorParameterValue _returnvalue "Edge Color" _output_get :!class /Script/Engine.MaterialInstanceDynamic)
  (bind _output_get_2 (LocalVariables|SetColor2 (Utilities|Struct|MakeLinearColor (Math|Random|RandomFloat) (Math|Random|RandomFloat) (Math|Random|RandomFloat) 1.0)))
  (Rendering|Material|SetVectorParameterValue _returnvalue "Color" _output_get_2 :!class /Script/Engine.MaterialInstanceDynamic)
  (bind _returnvalue_2 (Rendering|Material|CreateDynamicMaterialInstance (Variables|/Script/Engine.Character|GetMesh (Variables|Default|GetPlayerCaptureRef)) 1 0 "None" :!class /Script/Engine.PrimitiveComponent))
  (bind _output_get_3 (LocalVariables|SetColor3 (Utilities|Struct|MakeLinearColor (Math|Random|RandomFloat) (Math|Random|RandomFloat) (Math|Random|RandomFloat) 1.0)))
  (Rendering|Material|SetVectorParameterValue _returnvalue_2 "Edge Color" _output_get_3 :!class /Script/Engine.MaterialInstanceDynamic)
  (bind _output_get_4 (LocalVariables|SetColor4 (Utilities|Struct|MakeLinearColor (Math|Random|RandomFloat) (Math|Random|RandomFloat) (Math|Random|RandomFloat) 1.0)))
  (Rendering|Material|SetVectorParameterValue _returnvalue_2 "Color" _output_get_4 :!class /Script/Engine.MaterialInstanceDynamic)
  (Variables|/Game/Blueprints/Saving/BP_SavedCustomizationData.BP_SavedCustomizationData_C|SetColor1 _customizationsavedata (LocalVariables|GetColor1))
  (Variables|/Game/Blueprints/Saving/BP_SavedCustomizationData.BP_SavedCustomizationData_C|SetColor2 _customizationsavedata (LocalVariables|GetColor2))
  (Variables|/Game/Blueprints/Saving/BP_SavedCustomizationData.BP_SavedCustomizationData_C|SetColor3 _customizationsavedata (LocalVariables|GetColor3))
  (Variables|/Game/Blueprints/Saving/BP_SavedCustomizationData.BP_SavedCustomizationData_C|SetColor4 _customizationsavedata (LocalVariables|GetColor4)))

(fn ChangeHat
  (params (Hat%20Name :type String))
  (bind _output_get (Variables|/Game/Blueprints/Saving/BP_SavedCustomizationData.BP_SavedCustomizationData_C|SetSavedHatName (Variables|Default|GetCustomizationSaveData) Hat%20Name))
  (switch string _output_get
    (:Default
      (Private|SetHatVisibility))
    (:Skull
      (Private|SetHatVisibility (Variables|/Game/Blueprints/BP_GummyBear.BP_GummyBear_C|GetSkullHat_Low (Variables|Default|GetPlayerCaptureRef))))
    (:Helmet
      (Private|SetHatVisibility (Variables|/Game/Blueprints/BP_GummyBear.BP_GummyBear_C|GetHelmet (Variables|Default|GetPlayerCaptureRef))))
    (:Viking%20Helmet
      (Private|SetHatVisibility (Variables|/Game/Blueprints/BP_GummyBear.BP_GummyBear_C|GetVikingHelmet (Variables|Default|GetPlayerCaptureRef))))))

(fn SetHatVisibility
  (params (Hat :type Static%20Mesh%20Component%20Object%20Reference))
  (for _array_element (Variables|Default|GetPlayerHats)
    (Rendering|SetVisibility _array_element false false))
  (bind _hat (LocalVariables|GetHat)
    (:then
      (Rendering|SetVisibility _hat true false))
    (:else)))

(fn SaveGame
  (SaveGame|SaveGametoSlot (Variables|Default|GetCustomizationSaveData) (Variables|Default|GetSaveFileName)))