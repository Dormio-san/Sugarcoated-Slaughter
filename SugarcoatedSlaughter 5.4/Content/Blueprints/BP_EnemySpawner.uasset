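; BP_EnemySpawner is an actor that reads how many enemies to spawn from the ragdoll game mode's difficulty data.
; On BeginPlay it retries every 0.2 seconds until that data is valid, then stores the count and its SpawnRadius sphere's radius.
; A disconnected loop would spawn BP_EnemyGummy_Child at random reachable points within that radius, but nothing triggers it, so no enemies spawn here.
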(event EventBeginPlay
  (bind _asgm_ragdoll_game (Utilities|Casting|CastToGM_RagdollGame (Game|GetGameMode)))
  (bind _difficultysavedata (Variables|/Game/Blueprints/GM_RagdollGame.GM_RagdollGame_C|GetDifficultySaveData _asgm_ragdoll_game :!label _label)
    (:then
      (Variables|Default|SetNumEnemiesToSpawn (Variables|/Game/Blueprints/Saving/BP_DifficultySettings.BP_DifficultySettings_C|GetNumEnemiesToSpawn _difficultysavedata))
      (Variables|Default|SetEnemySpawnRadius (Variables|/Script/Engine.SphereComponent|GetSphereRadius (Variables|Default|GetSpawnRadius))))
    (:else
      (Utilities|FlowControl|Delay 0.2)
      (goto _label))))

(fn ConstructionScript)