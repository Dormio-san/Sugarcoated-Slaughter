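; Child enemy gummy bear AI that randomizes its colors, weapon and hat, and takes its health from the difficulty save data.
; Each tick it sphere-traces along the equipped weapon's sockets to damage the player and turns its health bar toward the camera.
; Sighting the player or taking damage sets a blackboard flag, which a retriggerable delay clears after sight.
; Death ragdolls it, and the last child to die shows the end screen.
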(event OnSeePawn(PawnSensing)
  (params (Pawn :type Pawn%20Object%20Reference))
  (bind _blackboard (Utilities|GetEnemyBlackboard))
  (bind _ai_seenplayerbool (Variables|Private|Constant|GetAI_SeenPlayerBool))
  ;[0 0 0] Player sensing which leads to chasing, or not if the player is no longer sensed.
  ;;[1 0.4757 0.9041] When a pawn is seen, check if it is the gummy bear (main character). If it is, continue.
  (Utilities|Casting|CastToBP_GummyBear Pawn)
  (Utilities|FlowControl|Sequence
    (:then_0
      ;;[0.286 1 0.7239] First, set the player seen bool in the AI blackboard to true.
      (AI|Components|Blackboard|SetValueasBool _blackboard _ai_seenplayerbool true))
    (:then_1
      (Utilities|FlowControl|RetriggerableDelay (Variables|Private|Constant|GetOutOfSightResetTime))
      (AI|Components|Blackboard|SetValueasBool _blackboard _ai_seenplayerbool false))))

(event Custom|ChildLoseHealth
  (bind _damage (Variables|Default|GetDamage))
  (bind _mesh (Variables|Character|GetMesh))
  (if (Variables|Default|GetChildCanTakeDamage)
    (Variables|Default|SetChildCanTakeDamage false)
    (if (not (Variables|/Game/Blueprints/GM_RagdollGame.GM_RagdollGame_C|GetIsGameOver (Variables|Default|GetGMRef)))
      (if (Utilities|IsAudioSourceNotPlaying _damage)
        (Audio|Components|Audio|Play _damage 0.0))
      (bind _result (Math|Integer|DecrementInt (Variables|Default|GetChildHealth))
        (:%20%20
          (Variables|Default|SetChildHealth _result)
          (CallFunction|UpdateHealthBar)
          (AI|Components|Blackboard|SetValueasBool (Utilities|GetEnemyBlackboard) (Variables|Private|Constant|GetAI_SeenPlayerBool) true)
          (if (<= (Variables|Default|GetChildHealth) 0)
            (Collision|SetCollisionEnabled _mesh "QueryAndPhysics")
            (Physics|SetSimulatePhysics _mesh true)
            (Class|SkeletalMeshComponent|SetPhysicsBlendWeight _mesh 1.0)
            (bind _healthbarwidget (Variables|Default|GetHealthBarWidget)
              (:then
                (Components|DestroyComponent _healthbarwidget))
              (:else
                _))
            (Utilities|FlowControl|Delay (Variables|Private|Constant|GetEnemyDeathTime))
            (bind _outactors (Actor|GetAllActorsOfClass "BP_EnemyGummy_Child_C"))
            (if (not (>= (Utilities|Array|Length _outactors) 2))
              (Utilities|FlowControl|DoOnce false
                (:Completed
                  (Default|ShowEndScreen (Variables|Default|GetGMRef) true))))
            (Actor|DestroyActor self)))))
    (else
      (Utilities|FlowControl|Delay (Variables|Private|Constant|GetPlayerCooldown))
      (Variables|Default|SetChildCanTakeDamage true))))

(event Custom|ChildDifficultySettings
  ;[0.1309 0.2344 0.09345] Load the difficulty settings. If a reference is not valid, wait and then try again.
  (bind _gmref (Variables|Default|GetGMRef :!label _label)
    (:then
      (bind _difficultysavedata (Variables|/Game/Blueprints/GM_RagdollGame.GM_RagdollGame_C|GetDifficultySaveData _gmref)
        (:then
          (bind _output_get (Variables|Private|SetChildMaxHealth (Variables|/Game/Blueprints/Saving/BP_DifficultySettings.BP_DifficultySettings_C|GetEnemyHealth _difficultysavedata)))
          (Variables|Default|SetChildHealth _output_get))
        (:else
          (Utilities|FlowControl|Delay 0.2 :!label _label_2)
          (goto _label))))
    (:else
      (goto _label_2))))

(event EventBeginPlay
  (CallFunction|SetReferences)
  (BeginPlay|Private|RandomCustomization)
  (CallFunction|ActiveRagdoll)
  (CallFunction|ChildDifficultySettings)
  (Variables|Default|SetChild true))

(event EventActorBeginOverlap
  (params (OtherActor :type Actor%20Object%20Reference)))

(event EventActorEndOverlap
  (params (OtherActor :type Actor%20Object%20Reference)))

(event EventLoseHealth)

(event EventTick
  (params (DeltaSeconds :type Float%20%28single-precision%29))
  (bind (_start _end) (Utilities|ClubStartEnd))
  (bind (_start_2 _end_2) (Utilities|SwordStartEnd))
  (Private|HealthBarFacePlayer)
  (if (Variables|Private|GetChildClubEquipped)
    (Private|ChildHitDetect _start _end)
    (else
      (Private|ChildHitDetect _start_2 _end_2))))

(fn ConstructionScript
  (|CallParentFunction))

(fn UpdateHealthBar
  (Progress|SetPercent (Variables|/Game/Blueprints/HealthBars/WBP_HealthBar.WBP_HealthBar_C|GetHealthBar (Variables|Default|GetWBP_HealthBar)) (/ (Variables|Default|GetChildHealth) (Variables|Private|GetChildMaxHealth))))

(fn ActiveRagdoll
  (|CallParentFunction))

(fn SetReferences
  (|CallParentFunction))

(fn RandomCustomization
  ;[0 0 0] Give each AI a random color.
  (bind _returnvalue (Rendering|Material|CreateDynamicMaterialInstance (Variables|Character|GetMesh) 0 0 "None" :!class /Script/Engine.PrimitiveComponent))
  (Rendering|Material|SetVectorParameterValue _returnvalue "Edge Color" (Utilities|Struct|MakeLinearColor (Math|Random|RandomFloat) (Math|Random|RandomFloat) (Math|Random|RandomFloat) 1.0) :!class /Script/Engine.MaterialInstanceDynamic)
  (Rendering|Material|SetVectorParameterValue _returnvalue "Color" (Utilities|Struct|MakeLinearColor (Math|Random|RandomFloat) (Math|Random|RandomFloat) (Math|Random|RandomFloat) 1.0) :!class /Script/Engine.MaterialInstanceDynamic)
  (bind _returnvalue_2 (Rendering|Material|CreateDynamicMaterialInstance (Variables|Character|GetMesh) 1 0 "None" :!class /Script/Engine.PrimitiveComponent))
  (Rendering|Material|SetVectorParameterValue _returnvalue_2 "Edge Color" (Utilities|Struct|MakeLinearColor (Math|Random|RandomFloat) (Math|Random|RandomFloat) (Math|Random|RandomFloat) 1.0) :!class /Script/Engine.MaterialInstanceDynamic)
  (Rendering|Material|SetVectorParameterValue _returnvalue_2 "Color" (Utilities|Struct|MakeLinearColor (Math|Random|RandomFloat) (Math|Random|RandomFloat) (Math|Random|RandomFloat) 1.0) :!class /Script/Engine.MaterialInstanceDynamic)
  ;[0 0 0] Give each AI a random weapon.
  (switch string (.OutItem (Utilities|Array|Random (Variables|Default|GetWeaponNames)))
    (:Default
      (Components|StaticMesh|SetStaticMesh (Variables|Default|GetEquippedWeapon) 0)
      (Components|StaticMesh|SetStaticMesh (Variables|Default|GetSwordWeapon) 0)
      (Variables|Private|SetChildClubEquipped false))
    (:Sword
      (Components|StaticMesh|SetStaticMesh (Variables|Default|GetSwordWeapon) "/Game/Art/Sword/sword_low.sword_low")
      (Components|StaticMesh|SetStaticMesh (Variables|Default|GetEquippedWeapon) 0)
      (Variables|Private|SetChildClubEquipped false))
    (:Club
      (Components|StaticMesh|SetStaticMesh (Variables|Default|GetEquippedWeapon) "/Game/Art/Props/Club.Club")
      (Components|StaticMesh|SetStaticMesh (Variables|Default|GetSwordWeapon) 0)
      (Variables|Private|SetChildClubEquipped true))
    (:Spear
      (Components|StaticMesh|SetStaticMesh (Variables|Default|GetEquippedWeapon) 0)
      (Components|StaticMesh|SetStaticMesh (Variables|Default|GetSwordWeapon) "/Game/Art/Props/spear_low.spear_low")
      (Variables|Private|SetChildClubEquipped false)))
  (Variables|Default|SetPlayerHats (Utilities|Array|MakeArray (Variables|Default|GetSkullHat_Low) (Variables|Default|GetHelmet) (Variables|Default|GetVikingHelmet)))
  ;[0 0 0] Give each AI a random hat.
  (switch string (.OutItem (Utilities|Array|Random (Variables|Default|GetHatNames)))
    (:Default
      (CallFunction|SetHatVisibility))
    (:Skull
      (CallFunction|SetHatVisibility (Variables|Default|GetSkullHat_Low)))
    (:Helmet
      (CallFunction|SetHatVisibility (Variables|Default|GetHelmet)))
    (:Viking%20Helmet
      (CallFunction|SetHatVisibility (Variables|Default|GetVikingHelmet)))))

(fn HealthBarFacePlayer
  (bind _healthbarwidget (Variables|Default|GetHealthBarWidget)
    (:then
      (Transformation|SetWorldRotation _healthbarwidget (Math|Rotator|FindLookatRotation (Transformation|GetWorldLocation _healthbarwidget) (Transformation|GetWorldLocation (Variables|/Script/Engine.PlayerCameraManager|GetTransformComponent (Game|GetPlayerCameraManager 0)))) false false))
    (:else)))

(fn ChildHitDetect
  (params (Start :type Vector) (End :type Vector))
  (bind (_outhit _returnvalue) (Collision|SphereTraceForObjects Start End 1e+01 (Utilities|Array|MakeArray "ObjectTypeQuery3") false 0 "None"))
  (if _returnvalue
    (bind _asbp_gummy_bear (Utilities|Casting|CastToBP_GummyBear (.HitActor (Collision|BreakHitResult _outhit))))
    (Default|LoseHealth _asbp_gummy_bear)))